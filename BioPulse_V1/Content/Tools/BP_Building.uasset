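; Procedural building tool that assembles static mesh pieces into a repeated 3D grid in the Construction Script.
; For each STBuilding entry, the CascadeLop macro loops over NombreMesh counts on X, Y and Z, spacing copies by TailleMesh from the entry's location.
; Each copy becomes its own Static Mesh Component with the entry's rotation, scale times ScaleMesh, and a dynamic instance of a randomly picked material on slot 0.
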(event EventBeginPlay)

(event Collision|EventActorBeginOverlap
  (params (OtherActor :type Actor%20Object%20Reference)))

(event EventTick
  (params (DeltaSeconds :type Float%20%28single-precision%29)))

(fn ConstructionScript
  (for _array_element (Variables|Default|GetST_Building)
    (bind (_returnx _returny _returnz) (Utilities|CascadeLop (.x (.Location (Math|Transform|BreakTransform (.Transform (Utilities|Struct|BreakST_Building _array_element))))) (.y (.Location (Math|Transform|BreakTransform (.Transform (Utilities|Struct|BreakST_Building _array_element))))) (.z (.Location (Math|Transform|BreakTransform (.Transform (Utilities|Struct|BreakST_Building _array_element))))))
      (:LoopBody
        (bind _returnvalue (AddComponent|AddStaticMeshComponent false (Math|Transform|MakeTransform (Math|Vector|MakeVector _returnx _returny _returnz) (.Rotation (Math|Transform|BreakTransform (.Transform (Utilities|Struct|BreakST_Building _array_element)))) (* (.Scale (Math|Transform|BreakTransform (.Transform (Utilities|Struct|BreakST_Building _array_element)))) (Variables|Default|GetScale_Mesh)))))
        (Components|StaticMesh|SetStaticMesh _returnvalue (.StaticMesh (Utilities|Struct|BreakST_Building _array_element)))
        (bind _returnvalue_2 (Rendering|Material|CreateDynamicMaterialInstance _returnvalue 0 (.OutItem (Utilities|Array|Random (.Material (Utilities|Struct|BreakST_Building _array_element)))) "None" :!class /Script/Engine.PrimitiveComponent))
        (Rendering|Material|SetMaterial _returnvalue 0 _returnvalue_2)))))

(fn Multiplication
  (params (AddX :type Float%20%28single-precision%29) (AddY :type Float%20%28single-precision%29) (AddZ :type Float%20%28single-precision%29))
  (bind (_returnx _returny _returnz) (Utilities|CascadeLop AddX AddY AddZ)
    (:LoopBody
      (return _returnx _returny _returnz))))