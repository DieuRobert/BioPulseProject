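; BP_Building1 is a building tool that assembles a repeated grid of meshes in its construction script.
; Each STBuilding entry gets its own instanced static mesh component, with a dynamic material instance created from that entry's material.
; The CascadeLop macro runs nested X/Y/Z loops over NombreMesh counts at TailleMesh spacing, adding an instance at each cell, offset and shaped by the entry's transform.
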(fn ConstructionScript
  (for _array_element (Variables|Default|GetST_Building)
    (bind _returnvalue (AddComponent|AddInstancedStaticMeshComponent false))
    (Components|StaticMesh|SetStaticMesh _returnvalue (.Mesh (Utilities|Struct|BreakST_building1 _array_element)))
    (bind _returnvalue_2 (Rendering|Material|CreateDynamicMaterialInstance _returnvalue 0 (.Material (Utilities|Struct|BreakST_building1 _array_element)) "None" :!class /Script/Engine.PrimitiveComponent))
    (Rendering|Material|SetMaterial _returnvalue 0 _returnvalue_2)
    (bind _transform (Utilities|CascadeLop (.x (.Location (Math|Transform|BreakTransform (.Transform (Utilities|Struct|BreakST_building1 _array_element))))) (.y (.Location (Math|Transform|BreakTransform (.Transform (Utilities|Struct|BreakST_building1 _array_element))))) (.z (.Location (Math|Transform|BreakTransform (.Transform (Utilities|Struct|BreakST_building1 _array_element))))))
      (:LoopBody
        (Components|InstancedStaticMesh|AddInstance _returnvalue (Math|Transform|MakeTransform _transform (.Rotation (Math|Transform|BreakTransform (.Transform (Utilities|Struct|BreakST_building1 _array_element)))) (.Scale (Math|Transform|BreakTransform (.Transform (Utilities|Struct|BreakST_building1 _array_element))))))))))