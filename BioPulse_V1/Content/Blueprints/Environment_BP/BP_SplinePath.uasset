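; Environment actor that moves an exterior whale mesh along a spline, started by the DoSmthing event or automatically on BeginPlay when flagged.
; A timeline, with play rate set from Speed, drives position and rotation by spline distance, with a yaw correction for the mesh.
; When the timeline finishes it sends the DoSmthing message again to repeat the path.
; A delayed 2D moan sound is guarded by a flag to play once.
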(event EventBeginPlay
  (if (Variables|Default|GetBeginPlau)
    (Class|BPIInteractions|DoSmthing(Message) self false false)))

(event EventDoSmthing
  (params (HasPass :type Boolean) (HasWeapon :type Boolean) (Actor :type Actor%20Object%20Reference))
  (bind _spline (Variables|Default|GetSpline))
  (Components|Timeline|SetPlayRate (Variables|Default|GetTimeline_0) (/ 1.0 (Variables|Default|GetSpeed)))
  (Utilities|FlowControl|Sequence
    (:then_0
      (bind _newtrack_0 (Timeline|Timeline_0 SetNewTime)
        (:Update
          (Variables|Default|SetAlpha _newtrack_0)
          (Transformation|SetRelativeLocationAndRotation (Variables|Default|GetExterieur_wildLife_whale) (Spline|GetLocationatDistanceAlongSpline _spline (Math|Float|Lerp 0.0 (Spline|GetSplineLength (Variables|Default|GetSpline)) (Variables|Default|GetAlpha)) "Local") (Math|Rotator|MakeRotator (.roll (Spline|GetRotationatDistanceAlongSpline _spline (Math|Float|Lerp 0.0 (Spline|GetSplineLength (Variables|Default|GetSpline)) (Variables|Default|GetAlpha)) "Local")) (.pitch (Spline|GetRotationatDistanceAlongSpline _spline (Math|Float|Lerp 0.0 (Spline|GetSplineLength (Variables|Default|GetSpline)) (Variables|Default|GetAlpha)) "Local")) (+ (.yaw (Spline|GetRotationatDistanceAlongSpline _spline (Math|Float|Lerp 0.0 (Spline|GetSplineLength (Variables|Default|GetSpline)) (Variables|Default|GetAlpha)) "Local")) -9e+01)) false false))
        (:Finished
          (Class|BPIInteractions|DoSmthing(Message) self false false))))
    (:then_1
      (Timeline|Timeline_0 Play))
    (:then_2
      (if (not (Variables|Default|GetDidMoan))
        (Utilities|FlowControl|Delay (Variables|Default|GetTimeBeforeSound))
        (Audio|PlaySound2D (Variables|Default|GetSound) 1.5 1.0 0.0 0 (Game|GetPlayerController 0) false)
        (Variables|Default|SetDidMoan true)))))

(fn ConstructionScript)