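; BP_Notes is an interactable note actor that displays its text or page in a W_Notes widget.
; NumNote selects the mesh material in the construction script and is passed to the widget as the note to show.
; DoSmthing opens the widget if the passed actor is PC_FirstPerson, then, regardless of that cast, shows the mouse cursor and disables player input.
; The Rrr overlap component toggles the mesh's custom depth stencil value as the player enters or leaves.
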(event OnComponentBeginOverlap(rrr)
  (params (OverlappedComponent :type Primitive%20Component%20Object%20Reference) (OtherActor :type Actor%20Object%20Reference) (OtherComp :type Primitive%20Component%20Object%20Reference) (OtherBodyIndex :type Integer) (bFromSweep :type Boolean) (SweepResult :type Hit%20Result%20Structure%20%28by%20ref%29))
  (if (== OtherActor (Game|GetPlayerCharacter 0))
    (Rendering|SetCustomDepthStencilValue (Variables|Default|GetNotes) 2)))

(event OnComponentEndOverlap(rrr)
  (params (OverlappedComponent :type Primitive%20Component%20Object%20Reference) (OtherActor :type Actor%20Object%20Reference) (OtherComp :type Primitive%20Component%20Object%20Reference) (OtherBodyIndex :type Integer))
  (if (== OtherActor (Game|GetPlayerCharacter 0))
    (Rendering|SetCustomDepthStencilValue (Variables|Default|GetNotes) 0)))

(event EventDoSmthing
  (params (HasPass :type Boolean) (HasWeapon :type Boolean) (Actor :type Actor%20Object%20Reference))
  (bind _returnvalue (Game|GetPlayerController 0))
  (CallFunction|ShowNote Actor)
  (Variables|/Script/Engine.PlayerController|SetbShowMouseCursor _returnvalue true)
  (Input|DisableInput (Game|GetPlayerCharacter 0) _returnvalue))

(fn ConstructionScript
  (Rendering|Material|SetMaterial (Variables|Default|GetNotes) 0 (Utilities|Array|Get(acopy) (.Materials (Utilities|Struct|BreakST_notes (Variables|Default|GetStructNotes))) (Variables|Default|GetNumNote))))

(fn ShowNote
  (params (Object :type Object%20Object%20Reference))
  (Utilities|Casting|CastToPC_FirstPerson Object)
  (bind _returnvalue (UserInterface|CreateWidget "/Game/Blueprints/UI/W_Notes.W_Notes_C"))
  (Variables|/Game/Blueprints/UI/W_Notes.W_Notes_C|SetNoteToShow _returnvalue (Variables|Default|GetNumNote))
  (UserInterface|Viewport|AddtoViewport _returnvalue 0))