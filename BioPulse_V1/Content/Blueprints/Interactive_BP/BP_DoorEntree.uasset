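; BP_DoorEntree is an interactive entrance door that opens once, only when triggered with a weapon.
; Its interaction event rotates the root's yaw through the OuverturePorte timeline while playing a creak sound at the door mesh.
; When the timeline finishes in Survival mode, it aggroes every Chrosome in CHChrosomes.
; The Rrr overlap toggles custom depth stencil on the door to highlight it for the nearby player while closed.
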(event OnComponentBeginOverlap(rrr)
  (params (OverlappedComponent :type Primitive%20Component%20Object%20Reference) (OtherActor :type Actor%20Object%20Reference) (OtherComp :type Primitive%20Component%20Object%20Reference) (OtherBodyIndex :type Integer) (bFromSweep :type Boolean) (SweepResult :type Hit%20Result%20Structure%20%28by%20ref%29))
  (if (and (Variables|Default|GetIsClose) (== OtherActor (Game|GetPlayerCharacter 0)))
    (Rendering|SetCustomDepthStencilValue (Variables|Default|Getcouloir_porte_middle) 2)))

(event OnComponentEndOverlap(rrr)
  (params (OverlappedComponent :type Primitive%20Component%20Object%20Reference) (OtherActor :type Actor%20Object%20Reference) (OtherComp :type Primitive%20Component%20Object%20Reference) (OtherBodyIndex :type Integer))
  (if (== OtherActor (Game|GetPlayerCharacter 0))
    (Rendering|SetCustomDepthStencilValue (Variables|Default|Getcouloir_porte_middle) 0)))

(event EventDoSmthing
  (params (HasPass :type Boolean) (HasWeapon :type Boolean) (Actor :type Actor%20Object%20Reference))
  (if (and HasWeapon (Variables|Default|GetIsClose))
    (Variables|Default|SetIsClose false)
    (Utilities|FlowControl|Sequence
      (:then_0
        (bind _ouverture (Timeline|Ouverture%20porte Play)
          (:Update
            (Transformation|SetWorldRotation (Variables|Default|GetDefaultSceneRoot) (Math|Rotator|MakeRotator 0.0 0.0 _ouverture) false false))
          (:Finished
            ;[1 1 1] Aggro Chrosomes
            (switch Utilities|FlowControl|Switch|SwitchonE_GameMode (Variables|Default|Getgamemode)
              (:NewEnumerator0
                (for _array_element (Variables|Default|GetCH%20chrosomes)
                  (Default|DoSmthing _array_element false false _array_element)))))))
      (:then_1
        (Audio|PlaySoundatLocation "/Game/Assets/Media/Audio/Sons_asset/WAV_DoorCrrrrr.WAV_DoorCrrrrr" (Transformation|GetWorldLocation (Variables|Default|Getcouloir_porte_middle)) "0, 0, 0" 1.0 1.0 0.0 0 0 0)))))

(fn ConstructionScript)