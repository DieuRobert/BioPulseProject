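; One-shot "inner voice" trigger that shows a line of floating text while playing a matching 2D voice sound.
; It fires on BeginPlay if flagged, otherwise on the player character's first overlap.
; A timeline fades the text color in, then the text hides after a set duration.
; Construction builds the collision box and sets the text; text and sound are picked by index from shared arrays.
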(event Collision|EventActorBeginOverlap
  (params (OtherActor :type Actor%20Object%20Reference))
  (bind _textrender (Variables|Default|GetTextRender))
  ;[1 1 1] SetVisibility
  (if (and (== OtherActor (Game|GetPlayerCharacter 0)) (not (Variables|Default|GetTriggered)))
    (Utilities|FlowControl|Sequence
      (:then_0
        (Variables|Default|SetTriggered true)
        (Rendering|SetVisibility _textrender true false)
        (bind _alpha (Timeline|fade%20in Play)
          (:Update
            (Rendering|Components|TextRender|SetTextRenderColor _textrender (Math|Conversions|ToColor(LinearColor) (Math|Conversions|ToLinearColor(Float) _alpha))))
          (:Finished
            (Utilities|FlowControl|Delay (Variables|Default|GetDurationText))
            (Rendering|SetVisibility _textrender false false))))
      (:then_1
        ;[1 1 1] PlaySound 2D
        (Audio|PlaySound2D (Utilities|Array|Get(acopy) (Utilities|Struct|BreakST_inHeadVoices (Variables|Default|GetST_Sound)) (Variables|Default|GetNum_Sound)) 1.0 1.0 0.0 0 0 false)))))

(event EventBeginPlay
  (bind _textrender (Variables|Default|GetTextRender))
  (Rendering|SetVisibility (Variables|Default|GetTextRender) false false)
  ;[1 1 1] SetVisibility
  (if (Variables|Default|GetBeginPlay?)
    (Utilities|FlowControl|Sequence
      (:then_0
        (Variables|Default|SetTriggered true)
        (Rendering|SetVisibility _textrender true false)
        (bind _alpha (Timeline|fade%20in Play)
          (:Update
            (Rendering|Components|TextRender|SetTextRenderColor _textrender (Math|Conversions|ToColor(LinearColor) (Math|Conversions|ToLinearColor(Float) _alpha))))
          (:Finished
            (Utilities|FlowControl|Delay (Variables|Default|GetDurationText))
            (Rendering|SetVisibility _textrender false false))))
      (:then_1
        ;[1 1 1] PlaySound 2D
        (Audio|PlaySound2D (Utilities|Array|Get(acopy) (Utilities|Struct|BreakST_inHeadVoices (Variables|Default|GetST_Sound)) (Variables|Default|GetNum_Sound)) 1.0 1.0 0.0 0 0 false)))))

(fn ConstructionScript
  ;[1 1 1] SetText
  (Rendering|Components|TextRender|SetText (Variables|Default|GetTextRender) (Utilities|Array|Get(acopy) (Utilities|Struct|BreakST_WrittenVoices (Variables|Default|GetST_Text)) (Variables|Default|GetNum_Text)))
  (AddComponent|AddBoxComponent false (Variables|Default|GetCollisionBox)))