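; BP_Pass is an interactive pickup that grants the first-person player a pass.
; DoSmthing, when its HasWeapon input is true, sets HasPass on PC_FirstPerson, prints a debug string and destroys the actor.
; Overlapping the Rrr component switches the Pass component's custom depth stencil while the player is inside, as used for highlighting.
; A ShowNote function, not called within this Blueprint, displays its Note in a W_Notes widget.
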(event OnComponentBeginOverlap(rrr)
  (params (OverlappedComponent :type Primitive%20Component%20Object%20Reference) (OtherActor :type Actor%20Object%20Reference) (OtherComp :type Primitive%20Component%20Object%20Reference) (OtherBodyIndex :type Integer) (bFromSweep :type Boolean) (SweepResult :type Hit%20Result%20Structure%20%28by%20ref%29))
  (if (== OtherActor (Game|GetPlayerCharacter 0))
    (Rendering|SetCustomDepthStencilValue (Variables|Default|GetPass) 2)))

(event OnComponentEndOverlap(rrr)
  (params (OverlappedComponent :type Primitive%20Component%20Object%20Reference) (OtherActor :type Actor%20Object%20Reference) (OtherComp :type Primitive%20Component%20Object%20Reference) (OtherBodyIndex :type Integer))
  (if (== OtherActor (Game|GetPlayerCharacter 0))
    (Rendering|SetCustomDepthStencilValue (Variables|Default|GetPass) 0)))

(event EventDoSmthing
  (params (HasPass :type Boolean) (HasWeapon :type Boolean) (Actor :type Actor%20Object%20Reference))
  (if HasWeapon
    (bind _aspc_first_person (Utilities|Casting|CastToPC_FirstPerson Actor))
    (Variables|/Game/Blueprints/PC_FirstPerson.PC_FirstPerson_C|SetHasPass _aspc_first_person true)
    (Development|PrintString "G LePaçe")
    (Actor|DestroyActor)))

(fn ConstructionScript)

(fn ShowNote
  (params (Object :type Object%20Object%20Reference))
  (Utilities|Casting|CastToPC_FirstPerson Object)
  (bind _returnvalue (UserInterface|CreateWidget "/Game/Blueprints/UI/W_Notes.W_Notes_C"))
  (bind _asw_notes (Utilities|Casting|CastToW_Notes _returnvalue))
  (Variables|/Game/Blueprints/UI/W_Notes.W_Notes_C|SetNoteToShow _asw_notes (Variables|Default|GetNote))
  (UserInterface|Viewport|AddtoViewport _returnvalue 0))