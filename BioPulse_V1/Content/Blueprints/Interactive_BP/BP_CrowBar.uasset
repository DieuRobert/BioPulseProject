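; Interactive crowbar pickup that gives the first-person player a crowbar.
; Its DoSmthing event casts the passed actor to PC_FirstPerson, calls GetCrowbar and destroys the pickup.
; The construction script adds a box component with overlap events enabled.
; Player overlap sets the mesh's custom depth stencil value, and BeginPlay runs the same check after a long delay, with no reset on leaving.
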(event Collision|EventActorBeginOverlap
  (params (OtherActor :type Actor%20Object%20Reference))
  (if (== OtherActor (Game|GetPlayerCharacter 0))
    (Rendering|SetCustomDepthStencilValue (Variables|Default|GetCrowBar) 2)))

(event EventDoSmthing
  (params (HasPass :type Boolean) (HasWeapon :type Boolean) (Actor :type Actor%20Object%20Reference))
  (if true
    (bind _aspc_first_person (Utilities|Casting|CastToPC_FirstPerson Actor))
    (Default|GetCrowbar _aspc_first_person)
    (Actor|DestroyActor)))

(event EventBeginPlay
  (Utilities|FlowControl|Delay 1.2e+02)
  (if (== (stale Collision|EventActorBeginOverlap OtherActor) (Game|GetPlayerCharacter 0))
    (Rendering|SetCustomDepthStencilValue (Variables|Default|GetCrowBar) 2)))

(fn ConstructionScript
  (bind _returnvalue (AddComponent|AddBoxComponent false (Variables|Default|GetCollisionBox)))
  (Variables|/Script/Engine.PrimitiveComponent|SetbGenerateOverlapEvents _returnvalue true))