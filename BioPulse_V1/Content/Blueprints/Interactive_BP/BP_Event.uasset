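; BP_Event is a one-shot trigger box that fires optional effects when the player character, with first tag "IsPlaying", overlaps it.
; It sets a Triggered flag, then runs three independently toggled effects in sequence.
; These damage the first-person player, call DoSmthing on every actor in the Chrosomes and Whales arrays, and play an indexed in-head voice as 2D sound.
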(event OnComponentBeginOverlap(Box)
  (params (OverlappedComponent :type Primitive%20Component%20Object%20Reference) (OtherActor :type Actor%20Object%20Reference) (OtherComp :type Primitive%20Component%20Object%20Reference) (OtherBodyIndex :type Integer) (bFromSweep :type Boolean) (SweepResult :type Hit%20Result%20Structure%20%28by%20ref%29))
  (bind _returnvalue (Game|GetPlayerCharacter 0))
  ;[1 1 1] If player and if not triggered
  (if (Math|Boolean|ANDBoolean (== OtherActor _returnvalue) (not (Variables|Default|GetTriggered)) (Utilities|Name|Equal(Name) (Utilities|Array|Get(acopy) (Variables|/Script/Engine.Actor|GetTags _returnvalue)) "IsPlaying"))
    (Utilities|FlowControl|Sequence
      (:then_0
        (Variables|Default|SetTriggered true))
      (:then_1
        (if (Variables|Default|GetDoDamage)
          (bind _aspc_first_person (Utilities|Casting|CastToPC_FirstPerson OtherActor))
          (Default|TakeDamage _aspc_first_person (Variables|Default|GetDamage))))
      (:then_2
        (if (Variables|Default|GetDoTriggerEvent)
          (for _array_element (Variables|Default|GetChrosomes)
            (Default|DoSmthing _array_element false false _array_element))
          (for _array_element_2 (Variables|Default|GetWhales)
            (Default|DoSmthing _array_element_2 false false _array_element_2))))
      (:then_3
        ;[1 1 1] PlaySound 2D
        (if (Variables|Default|GetDoPlaySound)
          (Audio|PlaySound2D (Utilities|Array|Get(acopy) (Utilities|Struct|BreakST_inHeadVoices (Variables|Default|GetST_Sound)) (Variables|Default|GetNum_Sound)) 1.0 1.0 0.0 0 0 false))))))

(fn ConstructionScript)