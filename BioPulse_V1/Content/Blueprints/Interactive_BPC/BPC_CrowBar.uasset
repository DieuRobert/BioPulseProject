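; Interactive crowbar pickup actor that gives the first-person player a crowbar.
; Its DoSmthing event casts the passed Player to PC_FirstPerson, calls GetCrowbar on it, then destroys the pickup.
; A separate ShowNote function creates a W_Notes widget showing the Note variable, but nothing in this file calls it.
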(event EventDoSmthing
  (params (HasPass :type Boolean) (HasWeapon :type Boolean) (Player :type Actor%20Object%20Reference))
  (if true
    (bind _aspc_first_person (Utilities|Casting|CastToPC_FirstPerson Player))
    (Default|GetCrowbar _aspc_first_person)
    (Actor|DestroyActor)))

(fn ConstructionScript)

(fn ShowNote
  (params (Object :type Object%20Object%20Reference))
  (Utilities|Casting|CastToPC_FirstPerson Object)
  (bind _returnvalue (UserInterface|CreateWidget "/Game/Blueprints/UI/W_Notes.W_Notes_C"))
  (bind _asw_notes (Utilities|Casting|CastToW_Notes _returnvalue))
  (Variables|/Game/Blueprints/UI/W_Notes.W_Notes_C|SetNoteToShow _asw_notes (Variables|Default|GetNote))
  (UserInterface|Viewport|AddtoViewport _returnvalue 0))