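; Punching bag Blueprint (sac de frappes) that takes damage until destroyed and also hurts the player on contact.
; TakeDamage lowers Health and prints it, then at zero or below sets IsDead, prints a French death message and destroys the actor.
; Overlapping its Box casts the other actor to PC_FirstPerson and calls that actor's TakeDamage with a fixed amount.
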(event OnComponentBeginOverlap(Box)
  (params (OverlappedComponent :type Primitive%20Component%20Object%20Reference) (OtherActor :type Actor%20Object%20Reference) (OtherComp :type Primitive%20Component%20Object%20Reference) (OtherBodyIndex :type Integer) (bFromSweep :type Boolean) (SweepResult :type Hit%20Result%20Structure%20%28by%20ref%29))
  (bind _aspc_first_person (Utilities|Casting|CastToPC_FirstPerson OtherActor))
  (Default|TakeDamage _aspc_first_person 1e+02))

(event EventTakeDamage
  (params (TakeDamage :type Float%20%28single-precision%29))
  (Utilities|FlowControl|Sequence
    (:then_0
      ;[1 1 1] degats
      (bind _output_get (Variables|Default|SetHealth (- (Variables|Default|GetHealth) TakeDamage)))
      (Development|PrintString (Utilities|String|ToString(Float) _output_get)))
    (:then_1
      ;[1 1 1] mort
      (if (<= (Variables|Default|GetHealth) 0.0)
        (Variables|Default|SetIsDead true)
        (Development|PrintString "Il est mort chef")
        (Actor|DestroyActor)))))

(fn ConstructionScript)