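; Behavior tree attack task for the CH_Chrosome AI character that, as wired, only changes its movement speed.
; On execute it casts the controlled pawn, raises or lowers max walk speed to a fixed value and immediately finishes successfully.
; A disconnected branch, which never runs, would check the IsPunching blackboard flag, call Attack, wait, then clear the flag before finishing.
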(event EventReceiveExecuteAI
  (params (OwnerController :type AI%20Controller%20Object%20Reference) (ControlledPawn :type Pawn%20Object%20Reference))
  (bind _asch_chrosome (Utilities|Casting|CastToCH_Chrosome ControlledPawn))
  (Variables|/Script/Engine.CharacterMovementComponent|SetMaxWalkSpeed (Variables|/Script/Engine.Character|GetCharacterMovement _asch_chrosome) 8e+02)
  (AI|BehaviorTree|FinishExecute true))