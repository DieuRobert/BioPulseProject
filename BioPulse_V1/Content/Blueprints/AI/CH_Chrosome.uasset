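; CH_Chrosome is an AI-controlled enemy that is forced to move toward the player and can be killed by damage.
; On BeginPlay it sets a boolean key on its Blackboard to trigger that movement.
; Its TakeDamage event subtracts from ChrosomeHealth and prints the result, then at zero or below flags IsDead, prints a death message and destroys the actor.
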(event EventBeginPlay
  ;[1 1 1] Force : move to player
  (AI|Components|Blackboard|SetValueasBool (AI|GetBlackboard self) (Variables|Default|Getbb_ref) true))

(event EventTakeDamage
  (params (TakeDamage :type Float%20%28single-precision%29))
  (Utilities|FlowControl|Sequence
    (:then_0
      ;[1 1 1] degats
      (bind _output_get (Variables|Default|SetChrosome_Health (- (Variables|Default|GetChrosome_Health) TakeDamage)))
      (Development|PrintString (Utilities|String|ToString(Float) _output_get)))
    (:then_1
      ;[1 1 1] mort
      (if (<= (Variables|Default|GetChrosome_Health) 0.0)
        (Variables|Default|SetIsDead true)
        (Development|PrintString "Il est mort chef")
        (Actor|DestroyActor)))))

(fn ConstructionScript)