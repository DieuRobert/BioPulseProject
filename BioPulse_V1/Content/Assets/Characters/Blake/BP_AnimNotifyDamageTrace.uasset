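; Anim notify state for Blake that deals damage during the animation window it covers.
; Each notify tick sphere-traces on the Visibility channel from the right middle finger socket, a short distance along the player camera's forward vector rather than the hand's direction.
; It sends TakeDamageMessage with fixed damage to the hit actor every tick, with no filter against repeat hits.
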(fn ReceivedNotifyTick
  (params (MeshComp :type Skeletal%20Mesh%20Component%20Object%20Reference) (Animation :type Anim%20Sequence%20Base%20Object%20Reference) (FrameDeltaTime :type Float%20%28single-precision%29))
  (bind _returnvalue (Transformation|GetSocketLocation MeshComp "MiddleFinger1_R"))
  (bind _returnvalue_2 (Game|GetPlayerCameraManager MeshComp))
  (bind _rootcomponent (Variables|/Script/Engine.Actor|GetRootComponent _returnvalue_2))
  (bind _returnvalue_3 (Math|Vector|GetForwardVector _rootcomponent))
  (bind _outhit (Collision|SphereTraceByChannel MeshComp _returnvalue (+ _returnvalue (* (Math|Vector|MakeVector (.x _returnvalue_3) (.y _returnvalue_3) (.z _returnvalue_3)) 1.5e+02)) 5.0 "TraceTypeQuery1" false 0 "None" true "(R=1.000000,G=0.000000,B=0.000000,A=1.000000)" "(R=0.000000,G=1.000000,B=0.000000,A=1.000000)" 2.0))
  (Class|BPIInteractions|TakeDamage(Message) (.HitActor (Collision|BreakHitResult _outhit)) 1e+01)
  (return true))